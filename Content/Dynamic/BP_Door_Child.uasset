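; BP_Door_Child is a door Blueprint child that swings its right door open and can stream in a new level.
; OpenDoor plays BaseDoorTimeline from the start, applying its RotateValue as DoorRight's relative yaw.
; When LoadNewLevel is set, each timeline update, rather than a one-time step, also calls a blocking LoadStreamLevel for NewLevelName, made visible after load.
; The construction script defers to the parent.
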(event EventBeginPlay
  (|CallParentFunction) ; This node is disabled and will not be called.\nDrag off pins to build functionality.
)

(event Collision|EventActorBeginOverlap
  (params (OtherActor :type Actor%20Object%20Reference))
  (|CallParentFunction OtherActor) ; This node is disabled and will not be called.\nDrag off pins to build functionality.
)

(event EventTick
  (params (DeltaSeconds :type Float%20%28single-precision%29))
  (|CallParentFunction DeltaSeconds) ; This node is disabled and will not be called.\nDrag off pins to build functionality.
)

(event EventOpenDoor
  (bind _rotatevalue (Timeline|BaseDoorTimeline PlayFromStart)
    (:Update
      (if (Variables|Default|GetbLoadNewLevel?)
        (Game|LoadStreamLevel(byName) (Variables|Default|GetNewLevelName) true true))
      (Transformation|SetRelativeRotation (Variables|Default|GetDoorRight) (Math|Rotator|MakeRotator 0.0 0.0 _rotatevalue) false false))))

(fn ConstructionScript
  (|CallParentFunction))